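; Behavior tree task that sends a BP_AI pawn to investigate around a blackboard location.
; It plays an enemy hit sound, triggers the pawn's EyePulse, then moves it to a random navigable point within InvestigateRadius.
; The task clears the investigating flag and succeeds on arrival or after an InvestigateTime delay running alongside the move.
; A failed move sets the flag true and fails the task.
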(event `self.ReceiveExecuteAI`
  (params (OwnerController :type "AIController Object Reference") (ControlledPawn :type "Pawn Object Reference"))
  (bind _investigating_key (`self.Investigating Key`))
  (`GameplayStatics.PlaySoundAtLocation` "/Game/Audio/SC_Enemy_Hit.SC_Enemy_Hit" (`Actor.K2_GetActorLocation` ControlledPawn) (struct) 1.0 1.0 0.0 null null ControlledPawn null)
  (bind _asbp_ai (cast `/Game/Blueprints/BP_AI` ControlledPawn))
  (`/Game/Blueprints/BP_AI.Eye Pulse` _asbp_ai)
  (bind _randomlocation (`NavigationSystemV1.K2_GetRandomLocationInNavigableRadius` (`BTFunctionLibrary.GetBlackboardValueAsVector` (`self.Key`)) (`self.Investigate Radius`) null null))
  (`|AIMoveTo` ControlledPawn _randomlocation null 5.0 true
    (:`then`
      (`KismetSystemLibrary.Delay` (`self.Investigate Time`))
      (`BTFunctionLibrary.SetBlackboardValueAsBool` (`self.Investigating Key`))
      (`self.FinishExecute` true))
    (:`OnSuccess`
      (`BTFunctionLibrary.SetBlackboardValueAsBool` _investigating_key)
      (`self.FinishExecute` true))
    (:`OnFail`
      (`BTFunctionLibrary.SetBlackboardValueAsBool` _investigating_key true)
      (`self.FinishExecute` false))))