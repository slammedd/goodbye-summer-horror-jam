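; Enemy AI character that detects the player through PawnSensing and reacts to shotgun hits.
; Sightings set the "Can See Player" Blackboard key, which a retriggerable delay clears once sight has been lost for a set time.
; ShotgunHit decrements Health and plays hit effects, with a one-second cooldown between hits.
; Look-around events use chained timelines to turn the capsule's yaw one way, then the other.
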(event `self.ReceiveBeginPlay`
  (set `self.Blackboard` (`AIBlueprintHelperLibrary.GetBlackboard` (`AIBlueprintHelperLibrary.GetAIController` (`self.GetController`)))))

(event `Shotgun Hit`
  (params (`Hit Location` :type "Vector Structure"))
  (if (not (`self.Cooldown`))
    (`/Engine/EditorBlueprintResources/StandardMacros.DecrementInt` (`self.Health`)
      (:`  `
        (`NiagaraFunctionLibrary.SpawnSystemAtLocation` "/Game/VFX/NS_Enemy_Hit.NS_Enemy_Hit" `Hit Location`)
        (`GameplayStatics.PlaySoundAtLocation` "/Game/Audio/SC_Enemy_Hit.SC_Enemy_Hit" `Hit Location` (struct) 1.0 1.0 0.0 null null null null)
        (set `self.Cooldown` true)
        (`KismetSystemLibrary.Delay` 1.0)
        (set `self.Cooldown` false)))))

(event `self.PawnSensing.OnSeePawn`
  (params (Pawn :type "Pawn Object Reference"))
  (`|ExecutionSequence`
    (:`then_0`
      (cast `/Game/Blueprints/BP_FirstPersonCharacter` Pawn)
      (`BlackboardComponent.SetValueAsBool` (`self.Blackboard`) "Can See Player" true))
    (:`then_1`
      (`KismetSystemLibrary.RetriggerableDelay` (`self.AI Continue Persue After Loss Of Sight`))
      (`BlackboardComponent.SetValueAsBool` (`self.Blackboard`) "Can See Player" false))))

(event `AI Look Around 1`
  (bind _capsulecomponent (`self.CapsuleComponent`))
  (bind (_returnvalue_roll _returnvalue_pitch _returnvalue_yaw) (`KismetMathLibrary.BreakRotator` (`SceneComponent.K2_GetComponentRotation` _capsulecomponent)))
  (`Timeline|Rotation` :!via `PlayFromStart`
    (:`Update`
      (`SceneComponent.K2_SetWorldRotation` _capsulecomponent (`KismetMathLibrary.MakeRotator` _returnvalue_roll _returnvalue_pitch (`KismetMathLibrary.Lerp` _returnvalue_yaw (+ _returnvalue_yaw 25.0) (* (`GameplayStatics.GetWorldDeltaSeconds`) 0.5))) false false))
    (:`Finished`
      (`self.AI Look Around 2`))))

(event `AI Look Around 2`
  (bind _capsulecomponent (`self.CapsuleComponent`))
  (bind (_returnvalue_roll _returnvalue_pitch _returnvalue_yaw) (`KismetMathLibrary.BreakRotator` (`SceneComponent.K2_GetComponentRotation` _capsulecomponent)))
  (`Timeline|Timeline` :!via `PlayFromStart`
    (:`Update`
      (`SceneComponent.K2_SetWorldRotation` _capsulecomponent (`KismetMathLibrary.MakeRotator` _returnvalue_roll _returnvalue_pitch (`KismetMathLibrary.Lerp` _returnvalue_yaw (+ _returnvalue_yaw -25.0) (* (`GameplayStatics.GetWorldDeltaSeconds`) 0.5))) false false))))

(fn `UserConstructionScript`)