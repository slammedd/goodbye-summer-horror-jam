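; BP_Shotgun is an interactable physics shotgun that spends ammo to fire randomly cone-spread pellets from its muzzle socket, or dry-clicks when empty.
; Firing ejects a shell, triggers smoke, flash, shakes, ear ringing and HUD blur, then kicks the gun out of the player's hands.
; A timeline drives post-process vignette while sprint is disabled.
; Shots, dry clicks and throttled drop impacts report noise events of differing range.
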(event `self.ReceiveBeginPlay`
  (bind _outactors (`GameplayStatics.GetAllActorsOfClass` "/Script/Engine.PostProcessVolume"))
  (set `self.Post Process Volume` (`|GetArrayItem` _outactors)))

(event `/Game/Blueprints/BPI_Interactable.Interact`
  (bind _returnvalue (`self.K2_GetActorLocation`))
  (bind _staticmesh (`self.StaticMesh`))
  (bind _staticmesh_2 (`self.StaticMesh`))
  (if (> (`self.Ammo`) 0)
    (`/Engine/EditorBlueprintResources/StandardMacros.DecrementInt` (`self.Ammo`)
      (:`  `
        (`AISense_Hearing.ReportNoiseEvent` _returnvalue 1.0 null 2000.0)
        (`GameplayStatics.PlaySoundAtLocation` "/Game/Audio/SC_Shotgun_Shot.SC_Shotgun_Shot" _returnvalue (struct) 1.0 1.0 0.0 null null null null)
        (`|SpawnActorFromClass` "/Game/Blueprints/BP_Shotgun_Shell.BP_Shotgun_Shell_C" (`KismetMathLibrary.MakeTransform` (`SceneComponent.GetSocketLocation` (`self.StaticMesh`) "Eject Port")) "Undefined" "MultiplyWithRoot" null null)
        (`self.Fire Shotgun`)
        (`NiagaraFunctionLibrary.SpawnSystemAtLocation` "/Game/VFX/NS_Shotgun_Smoke.NS_Shotgun_Smoke" (`SceneComponent.GetSocketLocation` _staticmesh "Muzzle") (`SceneComponent.GetSocketRotation` _staticmesh "Muzzle"))
        (`self.Trigger Light`)
        (`LegacyCameraShake.StartLegacyCameraShake` (`GameplayStatics.GetPlayerCameraManager` 0) "/Game/Blueprints/BP_Shotgun_Shake.BP_Shotgun_Shake_C")
        (bind _asbp_first_person_character (cast `/Game/Blueprints/BP_FirstPersonCharacter` (`GameplayStatics.GetPlayerCharacter` 0)))
        (`/Game/UI/WB_Player_HUD.Shotgun Blur` (`/Game/Blueprints/BP_FirstPersonCharacter.HUD` _asbp_first_person_character))
        (`GameplayStatics.PlaySound2D` "/Game/Audio/SC_Ear_Ringing.SC_Ear_Ringing" 1.0 1.0 0.0 null null)
        (`/Game/Blueprints/BP_FirstPersonCharacter.Drop Object` _asbp_first_person_character)
        (`/Game/Blueprints/BP_FirstPersonCharacter.Reset Rotate` _asbp_first_person_character)
        (set `/Game/Blueprints/BP_FirstPersonCharacter.Can Sprint` false _asbp_first_person_character)
        (`PrimitiveComponent.AddImpulseAtLocation` _staticmesh_2 (`KismetMathLibrary.NegateVector` (* (`SceneComponent.GetForwardVector` _staticmesh_2) (`self.Backwards Impulse Force`))) (`SceneComponent.K2_GetComponentLocation` _staticmesh_2) "None")
        (`KismetSystemLibrary.Delay` 0.2)
        (`LegacyCameraShake.StartLegacyCameraShake` (`GameplayStatics.GetPlayerCameraManager` 0) "/Game/Blueprints/BP_Shotgun_Shock.BP_Shotgun_Shock_C")
        (bind (_direction _intensity) (`Timeline|Vignette Intensity` :!via `PlayFromStart`)
          (:`Update`
            (set `PostProcessVolume.Settings` (make `PostProcessSettings` :`VignetteIntensity` _intensity) (`self.Post Process Volume`)))
          (:`Finished`
            (set `/Game/Blueprints/BP_FirstPersonCharacter.Can Sprint` true _asbp_first_person_character)))))
    (else
      (`GameplayStatics.PlaySoundAtLocation` "/Game/Audio/SC_Shotgun_Empty.SC_Shotgun_Empty" _returnvalue (struct) 1.0 1.0 0.0 null null null null)
      (`AISense_Hearing.ReportNoiseEvent` _returnvalue 0.4 null 500.0))))

(event `Trigger Light`
  (bind _pointlight (`self.PointLight`))
  (`SceneComponent.SetVisibility` _pointlight true false)
  (`KismetSystemLibrary.Delay` 0.05)
  (`SceneComponent.SetVisibility` _pointlight false false))

(event `self.StaticMesh.OnComponentHit`
  (params (HitComponent :type "PrimitiveComponent Object Reference") (OtherActor :type "Actor Object Reference") (OtherComp :type "PrimitiveComponent Object Reference") (NormalImpulse :type "Vector Structure") (Hit :type "HitResult Structure (by ref)"))
  (bind _returnvalue (`self.K2_GetActorLocation`))
  (bind _returnvalue_2 (`KismetMathLibrary.VSize` NormalImpulse))
  (bind (_bblockinghit _binitialoverlap _time _distance _location _impactpoint _normal _impactnormal) (`GameplayStatics.BreakHitResult` Hit))
  (if (> _returnvalue_2 1500.0)
    (if (> _returnvalue_2 3000.0)
      (`NiagaraFunctionLibrary.SpawnSystemAtLocation` "/Game/VFX/NS_Generic_Impact_Smoke.NS_Generic_Impact_Smoke" _location (`KismetMathLibrary.MakeRotFromX` _impactnormal)))
    (`/Engine/EditorBlueprintResources/StandardMacros.DoOnce` false :!label _label
      (:`Completed`
        (`GameplayStatics.PlaySoundAtLocation` "/Game/Audio/SC_Shotgun_Drop.SC_Shotgun_Drop" _returnvalue (struct) 1.0 1.0 0.0 null null null null)
        (`AISense_Hearing.ReportNoiseEvent` _returnvalue 0.3 null 300.0)
        (`KismetSystemLibrary.Delay` 1.0)
        (goto _label :!via `Reset`)))))

(event `Fire Shotgun`
  (bind _staticmesh (`self.StaticMesh`))
  ;[1 1 1] Fire Shotgun
  (for _ (range 1 (+ (`self.Shot Amount`) 1))
    (`|SpawnActorFromClass` "/Game/Blueprints/BP_Shotgun_Pellet.BP_Shotgun_Pellet_C" (`KismetMathLibrary.MakeTransform` (`SceneComponent.GetSocketLocation` _staticmesh "Muzzle") (`self.Get Spray Angle` (`KismetMathLibrary.GetForwardVector` (`SceneComponent.GetSocketRotation` _staticmesh "Muzzle")) (`self.Max Angle`))) "Undefined" "MultiplyWithRoot" null null)))

(fn `Get Spray Angle`
  (params (`Muzzle Direction` :type "Vector Structure") (`Max Angle` :type "Float (double-precision)"))
  (returns (`Shot Rotation` :type "Rotator Structure"))
  (return (`KismetMathLibrary.MakeRotFromX` (`KismetMathLibrary.RandomUnitVectorInConeInDegrees` `Muzzle Direction` `Max Angle`))))

(fn `UserConstructionScript`)