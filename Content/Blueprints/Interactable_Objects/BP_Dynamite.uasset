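; Interactable dynamite prop that a lit BP_Lighter ignites on overlap, offering a possible win ending.
; Lighting starts the fuse effect and a timed explosion with camera shake, then either destroys the actor or, if CanWin is set, runs the player's HUD victory sequence.
; Hard physics hits play throttled impact sounds with AI noise, adding smoke on stronger ones, after a short startup delay.
; Direct interaction only shows the HUD cross icon.
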(event `/Game/Blueprints/BPI_Interactable.Interact`
  (bind _asbp_first_person_character (cast `/Game/Blueprints/BP_FirstPersonCharacter` (`GameplayStatics.GetPlayerCharacter` 0)))
  (`/Game/UI/WB_Player_HUD.Cross Icon` (`/Game/Blueprints/BP_FirstPersonCharacter.HUD` _asbp_first_person_character)))

(event `self.ReceiveBeginPlay`
  (`KismetSystemLibrary.Delay` 2.0)
  (set `self.Can Sound` true))

(event `self.StaticMesh.OnComponentHit`
  (params (HitComponent :type "PrimitiveComponent Object Reference") (OtherActor :type "Actor Object Reference") (OtherComp :type "PrimitiveComponent Object Reference") (NormalImpulse :type "Vector Structure") (Hit :type "HitResult Structure (by ref)"))
  (bind _returnvalue (`self.K2_GetActorLocation`))
  (bind _returnvalue_2 (`KismetMathLibrary.VSize` NormalImpulse))
  (bind (_bblockinghit _binitialoverlap _time _distance _location _impactpoint _normal _impactnormal) (`GameplayStatics.BreakHitResult` Hit))
  (if (`self.Can Sound`)
    (if (> _returnvalue_2 2000.0)
      (if (> _returnvalue_2 4000.0)
        (`NiagaraFunctionLibrary.SpawnSystemAtLocation` "/Game/VFX/NS_Generic_Impact_Smoke.NS_Generic_Impact_Smoke" _location (`KismetMathLibrary.MakeRotFromX` _impactnormal)))
      (`/Engine/EditorBlueprintResources/StandardMacros.DoOnce` false :!label _label
        (:`Completed`
          (`GameplayStatics.PlaySoundAtLocation` "/Game/Audio/SC_Generic_Impact.SC_Generic_Impact" _returnvalue (struct) 1.0 1.0 0.0 null null null null)
          (`AISense_Hearing.ReportNoiseEvent` _returnvalue 0.05 null 150.0)
          (`KismetSystemLibrary.Delay` 1.0)
          (goto _label :!via `Reset`))))))

(event `self.Box.OnComponentBeginOverlap`
  (params (OverlappedComponent :type "PrimitiveComponent Object Reference") (OtherActor :type "Actor Object Reference") (OtherComp :type "PrimitiveComponent Object Reference") (OtherBodyIndex :type Integer) (bFromSweep :type Boolean) (SweepResult :type "HitResult Structure (by ref)"))
  (bind _asbp_lighter (cast `/Game/Blueprints/Interactable_Objects/BP_Lighter` OtherActor))
  (if (`/Game/Blueprints/Interactable_Objects/BP_Lighter.Lighter On` _asbp_lighter)
    (`self.Light Dynamite`)))

(event `Light Dynamite`
  (bind _returnvalue (`SceneComponent.K2_GetComponentLocation` (`self.StaticMesh`)))
  (`PrimitiveComponent.SetCollisionEnabled` (`self.Box`) "NoCollision")
  (`ActorComponent.SetActive` (`self.Fire`) true false)
  (`GameplayStatics.PlaySoundAtLocation` "/Game/Audio/SC_Lit_Dynamite.SC_Lit_Dynamite" _returnvalue (struct) 1.0 1.0 0.0 null null null null)
  (`KismetSystemLibrary.Delay` 5.0)
  (`GameplayStatics.PlaySoundAtLocation` "/Game/Audio/SC_Dynamite_Explosion.SC_Dynamite_Explosion" _returnvalue (struct) 1.0 1.0 0.0 null null null null)
  (`NiagaraFunctionLibrary.SpawnSystemAtLocation` "/Game/VFX/NS_Explosion.NS_Explosion" _returnvalue)
  (if (`self.Can Win`)
    (bind _asbp_first_person_character (cast `/Game/Blueprints/BP_FirstPersonCharacter` (`GameplayStatics.GetPlayerCharacter` 0))
      (:`then`
        (set `/Game/Blueprints/BP_FirstPersonCharacter.Player Win` true _asbp_first_person_character)
        (`LegacyCameraShake.StartLegacyCameraShake` (`GameplayStatics.GetPlayerCameraManager` 0) "/Game/Blueprints/BP_Explosion_Shake.BP_Explosion_Shake_C")
        (`SceneComponent.SetVisibility` (`self.StaticMesh`) false false)
        (`ActorComponent.SetActive` (`self.Fire`) false false)
        (set `/Game/Blueprints/BP_FirstPersonCharacter.Can Move` false _asbp_first_person_character)
        (`KismetSystemLibrary.Delay` 3.0)
        (`/Game/Blueprints/BP_FirstPersonCharacter.Switch to UI Input` _asbp_first_person_character)
        (bind _hud (`/Game/Blueprints/BP_FirstPersonCharacter.HUD` _asbp_first_person_character))
        (`/Game/UI/WB_Player_HUD.Fade to Black` _hud)
        (`KismetSystemLibrary.Delay` 3.0)
        (`/Game/UI/WB_Player_HUD.Dynamite Win` _hud)
        (`KismetSystemLibrary.Delay` 3.0)
        (`/Game/UI/WB_Player_HUD.Fade Death Buttons` _hud))
      (:`CastFailed`
        (`KismetSystemLibrary.PrintString` "Hello")))
    (else
      (`LegacyCameraShake.StartLegacyCameraShake` (`GameplayStatics.GetPlayerCameraManager` 0) "/Game/Blueprints/BP_Explosion_Shake.BP_Explosion_Shake_C")
      (`self.K2_DestroyActor`))))

(fn `UserConstructionScript`)