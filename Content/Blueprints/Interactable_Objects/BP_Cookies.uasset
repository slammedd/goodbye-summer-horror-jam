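; BP_Cookies is an interactable cookies prop that reacts to physical impacts.
; Interacting with it only calls CrossIcon on the first-person character's HUD.
; After a short startup delay, mesh hits above an impulse threshold play a sound and report a faint, short-range noise event, throttled by a DoOnce with delayed reset.
; Harder hits also spawn Niagara smoke at the contact point, outside that throttle.
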(event `/Game/Blueprints/BPI_Interactable.Interact`
  (bind _asbp_first_person_character (cast `/Game/Blueprints/BP_FirstPersonCharacter` (`GameplayStatics.GetPlayerCharacter` 0)))
  (`/Game/UI/WB_Player_HUD.Cross Icon` (`/Game/Blueprints/BP_FirstPersonCharacter.HUD` _asbp_first_person_character)))

(event `self.ReceiveBeginPlay`
  (`KismetSystemLibrary.Delay` 2.0)
  (set `self.Can Sound` true))

(event `self.StaticMesh.OnComponentHit`
  (params (HitComponent :type "PrimitiveComponent Object Reference") (OtherActor :type "Actor Object Reference") (OtherComp :type "PrimitiveComponent Object Reference") (NormalImpulse :type "Vector Structure") (Hit :type "HitResult Structure (by ref)"))
  (bind _returnvalue (`self.K2_GetActorLocation`))
  (bind _returnvalue_2 (`KismetMathLibrary.VSize` NormalImpulse))
  (bind (_bblockinghit _binitialoverlap _time _distance _location _impactpoint _normal _impactnormal) (`GameplayStatics.BreakHitResult` Hit))
  (if (`self.Can Sound`)
    (if (> _returnvalue_2 2000.0)
      (if (> _returnvalue_2 4000.0)
        (`NiagaraFunctionLibrary.SpawnSystemAtLocation` "/Game/VFX/NS_Generic_Impact_Smoke.NS_Generic_Impact_Smoke" _location (`KismetMathLibrary.MakeRotFromX` _impactnormal)))
      (`/Engine/EditorBlueprintResources/StandardMacros.DoOnce` false :!label _label
        (:`Completed`
          (`GameplayStatics.PlaySoundAtLocation` "/Game/Audio/SC_Generic_Impact.SC_Generic_Impact" _returnvalue (struct) 1.0 1.0 0.0 null null null null)
          (`AISense_Hearing.ReportNoiseEvent` _returnvalue 0.05 null 150.0)
          (`KismetSystemLibrary.Delay` 1.0)
          (goto _label :!via `Reset`))))))

(fn `UserConstructionScript`)