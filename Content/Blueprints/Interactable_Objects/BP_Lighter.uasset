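; BP_Lighter is an interactable lighter that toggles its flame and point light, with a click sound and an AI noise event on each use.
; While lit, a Timeline drives flicker by easing light intensity toward a periodically randomized target.
; Hard mesh hits play a throttled impact sound and report noise, with smoke on stronger hits.
; Impact reactions stay disabled briefly after BeginPlay.
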(event `/Game/Blueprints/BPI_Interactable.Interact`
  (bind _returnvalue (`self.K2_GetActorLocation`))
  (bind _flame (`self.Flame`))
  (bind _pointlight (`self.PointLight`))
  (bind _pointlight_2 (`self.PointLight`))
  (`GameplayStatics.PlaySoundAtLocation` "/Game/Audio/SC_Lighter.SC_Lighter" _returnvalue (struct) 1.0 1.0 0.0 null null null null)
  (`AISense_Hearing.ReportNoiseEvent` _returnvalue 0.1 null 50.0)
  (if (`self.Lighter On`)
    (`ActorComponent.SetActive` _flame false false)
    (`SceneComponent.SetHiddenInGame` _pointlight true false)
    (set `self.Lighter On` false)
    (`Timeline|Timeline` :!via `Stop` :!label _label
      (:`Update`
        (`|ExecutionSequence`
          (:`then_0`
            (`LightComponent.SetIntensity` _pointlight_2 (`KismetMathLibrary.Lerp` (`LightComponentBase.Intensity` _pointlight_2) (`self.Target Intensity`) (* (`GameplayStatics.GetWorldDeltaSeconds`) (`self.Flicker Speed`)))))
          (:`then_1`
            (`KismetSystemLibrary.Delay` (`KismetMathLibrary.RandomFloatInRange` 0.05 0.15))
            (set `self.Target Intensity` (`KismetMathLibrary.RandomFloatInRange` 50.0 100.0))))))
    (else
      (`ActorComponent.SetActive` _flame true false)
      (`SceneComponent.SetHiddenInGame` _pointlight false false)
      (set `self.Lighter On` true)
      (goto _label :!via `PlayFromStart`))))

(event `self.ReceiveBeginPlay`
  (`KismetSystemLibrary.Delay` 2.0)
  (set `self.Can Sound` true))

(event `self.StaticMesh.OnComponentHit`
  (params (HitComponent :type "PrimitiveComponent Object Reference") (OtherActor :type "Actor Object Reference") (OtherComp :type "PrimitiveComponent Object Reference") (NormalImpulse :type "Vector Structure") (Hit :type "HitResult Structure (by ref)"))
  (bind _returnvalue (`self.K2_GetActorLocation`))
  (bind _returnvalue_2 (`KismetMathLibrary.VSize` NormalImpulse))
  (bind (_bblockinghit _binitialoverlap _time _distance _location _impactpoint _normal _impactnormal) (`GameplayStatics.BreakHitResult` Hit))
  (if (`self.Can Sound`)
    (if (> _returnvalue_2 2000.0)
      (if (> _returnvalue_2 4000.0)
        (`NiagaraFunctionLibrary.SpawnSystemAtLocation` "/Game/VFX/NS_Generic_Impact_Smoke.NS_Generic_Impact_Smoke" _location (`KismetMathLibrary.MakeRotFromX` _impactnormal)))
      (`/Engine/EditorBlueprintResources/StandardMacros.DoOnce` false :!label _label_2
        (:`Completed`
          (`GameplayStatics.PlaySoundAtLocation` "/Game/Audio/SC_Generic_Impact.SC_Generic_Impact" _returnvalue (struct) 1.0 1.0 0.0 null null null null)
          (`AISense_Hearing.ReportNoiseEvent` _returnvalue 0.05 null 150.0)
          (`KismetSystemLibrary.Delay` 1.0)
          (goto _label_2 :!via `Reset`))))))

(fn `UserConstructionScript`)