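; A physics-driven door that can start locked and makes AI-audible noise when unlocked, swung or closed.
; While locked, physics is off until a BP_Key with a matching code hits the door, which destroys the key and enables simulation.
; Each Tick checks velocity for fast swings and yaw for closing, using DoOnce gates to limit repeated sounds and noise events.
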(event `self.ReceiveBeginPlay`
  ;[1 1 1] Locked Door
  (set `self.Previous Rot` (`SceneComponent.RelativeRotation` (`self.Door`)))
  (if (`self.IsLocked`)
    (`PrimitiveComponent.SetSimulatePhysics` (`self.Door`) false)))

(event `self.Door.OnComponentHit`
  (params (HitComponent :type "PrimitiveComponent Object Reference") (OtherActor :type "Actor Object Reference") (OtherComp :type "PrimitiveComponent Object Reference") (NormalImpulse :type "Vector Structure") (Hit :type "HitResult Structure (by ref)"))
  (bind _returnvalue (`SceneComponent.K2_GetComponentLocation` (`self.Door`)))
  ;[1 1 1] Locked Door
  (if (`self.IsLocked`)
    (bind _asbp_key (cast `/Game/Blueprints/BP_Key` OtherActor))
    (if (== (`/Game/Blueprints/BP_Key.KeyCode` _asbp_key) (`self.DoorCode`))
      (`/Game/Blueprints/BP_Key.Destroy Key` _asbp_key)
      (`PrimitiveComponent.SetSimulatePhysics` (`self.Door`) true)
      (`GameplayStatics.PlaySoundAtLocation` "/Game/Audio/SC_Door_Unlock.SC_Door_Unlock" _returnvalue (struct) 1.0 1.0 0.0 null null null null)
      (`AISense_Hearing.ReportNoiseEvent` _returnvalue 0.2 null 100.0)
      (set `self.IsLocked` false))))

(event `self.ReceiveTick`
  (params (DeltaSeconds :type "Float (single-precision)"))
  (`self.Door Swing`)
  (`self.Door Close`))

(event `Door Close`
  (bind _returnvalue (`self.K2_GetActorLocation`))
  (bind _door (`self.Door`))
  (bind (_relativerotation_roll _relativerotation_pitch _relativerotation_yaw) (`KismetMathLibrary.BreakRotator` (`SceneComponent.RelativeRotation` _door)))
  (set `self.Previous Rot` (`SceneComponent.RelativeRotation` _door))
  (if (< _relativerotation_yaw 92.0)
    (`/Engine/EditorBlueprintResources/StandardMacros.DoOnce` true :!label _label
      (:`Completed`
        (`GameplayStatics.PlaySoundAtLocation` "/Game/Audio/SC_Door_Close.SC_Door_Close" _returnvalue (struct) 1.0 1.0 0.0 null null null null)
        (`AISense_Hearing.ReportNoiseEvent` _returnvalue 0.5 (`GameplayStatics.GetPlayerCharacter` 0) 300.0)))
    (else
      (goto _label :!via `Reset`))))

(event `Door Swing`
  (bind _returnvalue (`self.K2_GetActorLocation`))
  (if (> (`KismetMathLibrary.VSize` (`SceneComponent.GetComponentVelocity` (`self.Door`))) 350.0)
    (`/Engine/EditorBlueprintResources/StandardMacros.DoOnce` false :!label _label_2
      (:`Completed`
        (`GameplayStatics.PlaySoundAtLocation` "/Game/Audio/SC_Door_Swing.SC_Door_Swing" _returnvalue (struct) 1.0 1.0 0.0 null null null null)
        (`AISense_Hearing.ReportNoiseEvent` _returnvalue 0.5 (`GameplayStatics.GetPlayerCharacter` 0) 300.0)
        (`KismetSystemLibrary.Delay` 1.0)
        (goto _label_2 :!via `Reset`)))))

(fn `UserConstructionScript`)