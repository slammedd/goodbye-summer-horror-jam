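; BP_CabinetJoseph is a cabinet with a moving door that plays sounds and reports noise to AI.
; After a two-second startup delay, Tick checks door velocity for swings and relative yaw for closing.
; DoOnce gates prevent repeats: swing re-arms after a delay, while close starts closed and re-arms when the door opens past its threshold.
; Noise events name the player as instigator; the stored previous rotation is never read.
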(event `self.ReceiveBeginPlay`
  (set `self.Previous Rot` (`SceneComponent.RelativeRotation` (`self.Door`)))
  (`KismetSystemLibrary.Delay` 2.0)
  (set `self.Can Sound` true))

(event `self.ReceiveTick`
  (params (DeltaSeconds :type "Float (single-precision)"))
  (if (`self.Can Sound`)
    (`self.Door Swing`)
    (`self.Door Close`)))

(event `Door Close`
  (bind _returnvalue (`self.K2_GetActorLocation`))
  (bind _door (`self.Door`))
  (bind (_relativerotation_roll _relativerotation_pitch _relativerotation_yaw) (`KismetMathLibrary.BreakRotator` (`SceneComponent.RelativeRotation` _door)))
  (set `self.Previous Rot` (`SceneComponent.RelativeRotation` _door))
  (if (< _relativerotation_yaw 95.0)
    (`/Engine/EditorBlueprintResources/StandardMacros.DoOnce` true :!label _label
      (:`Completed`
        (`GameplayStatics.PlaySoundAtLocation` "/Game/Audio/SC_Door_Close.SC_Door_Close" _returnvalue (struct) 1.0 1.0 0.0 null null null null)
        (`AISense_Hearing.ReportNoiseEvent` _returnvalue 0.5 (`GameplayStatics.GetPlayerCharacter` 0) 300.0)))
    (else
      (goto _label :!via `Reset`))))

(event `Door Swing`
  (bind _returnvalue (`self.K2_GetActorLocation`))
  (if (> (`KismetMathLibrary.VSize` (`SceneComponent.GetComponentVelocity` (`self.Door`))) 500.0)
    (`/Engine/EditorBlueprintResources/StandardMacros.DoOnce` false :!label _label_2
      (:`Completed`
        (`GameplayStatics.PlaySoundAtLocation` "/Game/Audio/SC_Door_Swing.SC_Door_Swing" _returnvalue (struct) 1.0 1.0 0.0 null null null null)
        (`AISense_Hearing.ReportNoiseEvent` _returnvalue 0.5 (`GameplayStatics.GetPlayerCharacter` 0) 300.0)
        (`KismetSystemLibrary.Delay` 1.0)
        (goto _label_2 :!via `Reset`)))))

(fn `UserConstructionScript`)