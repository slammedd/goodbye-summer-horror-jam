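; Shotgun pellet actor that resolves its impact when its collision sphere hits something other than the first-person character.
; On a hit it disables collision and hides the visual sphere, then forwards the impact point to BP_AI's ShotgunHit for BPI_Enemy targets.
; Other surfaces get smoke and shard Niagara effects, an impact sound and an AI noise event attributed to the player.
; Only this non-enemy branch destroys the pellet, after a short delay.
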(event `self.Sphere1.OnComponentHit`
  (params (HitComponent :type "PrimitiveComponent Object Reference") (OtherActor :type "Actor Object Reference") (OtherComp :type "PrimitiveComponent Object Reference") (NormalImpulse :type "Vector Structure") (Hit :type "HitResult Structure (by ref)"))
  (bind (_bblockinghit _binitialoverlap _time _distance _location _impactpoint _normal _impactnormal) (`GameplayStatics.BreakHitResult` Hit))
  (bind _returnvalue (`KismetMathLibrary.MakeRotFromX` _impactnormal))
  (cast `/Game/Blueprints/BP_FirstPersonCharacter` OtherActor
    (:`CastFailed`
      (`PrimitiveComponent.SetCollisionEnabled` (`self.Sphere1`) "NoCollision")
      (`SceneComponent.SetVisibility` (`self.Sphere`) false false)
      (if (`KismetSystemLibrary.DoesImplementInterface` OtherActor "/Game/Blueprints/BPI_Enemy.BPI_Enemy_C")
        (bind _asbp_ai (cast `/Game/Blueprints/BP_AI` OtherActor))
        (`/Game/Blueprints/BP_AI.Shotgun Hit` _asbp_ai _impactpoint)
        (else
          (`NiagaraFunctionLibrary.SpawnSystemAtLocation` "/Game/VFX/NS_Pellet_Impact_Smoke.NS_Pellet_Impact_Smoke" _impactpoint _returnvalue)
          (`NiagaraFunctionLibrary.SpawnSystemAtLocation` "/Game/VFX/NS_Impact_Shards_Wall.NS_Impact_Shards_Wall" _impactpoint _returnvalue)
          (`GameplayStatics.PlaySoundAtLocation` "/Game/Audio/SC_Pellet_Impact.SC_Pellet_Impact" _impactpoint (struct) 1.0 1.0 0.0 null null null null)
          (`AISense_Hearing.ReportNoiseEvent` _impactpoint 0.3 (`GameplayStatics.GetPlayerCharacter` 0) 200.0)
          (`KismetSystemLibrary.Delay` 0.2)
          (`self.K2_DestroyActor`))))))

(fn `UserConstructionScript`)