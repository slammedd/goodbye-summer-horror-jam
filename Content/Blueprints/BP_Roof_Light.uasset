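; BP_Roof_Light is a roof light Blueprint whose static mesh can switch between its default look and a flicker material.
; BeginPlay caches the material in slot 0 as the default.
; The SwitchMaterial event compares the current material to that cached one and toggles between it and FlickerMaterial.
; Nothing in this Blueprint calls SwitchMaterial or changes any light component.
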(event `self.ReceiveBeginPlay`
  (set `self.Default Material` (`PrimitiveComponent.GetMaterial` (`self.StaticMesh`) 0)))

(event `/Game/Blueprints/BPI_Light_Identifier.Switch Material`
  (bind _staticmesh (`self.StaticMesh`))
  (if (== (`PrimitiveComponent.GetMaterial` (`self.StaticMesh`) 0) (`self.Default Material`))
    (`PrimitiveComponent.SetMaterial` _staticmesh 0 (`self.Flicker Material`))
    (else
      (`PrimitiveComponent.SetMaterial` _staticmesh 0 (`self.Default Material`)))))

(fn `UserConstructionScript`)